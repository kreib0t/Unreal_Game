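; Base game state that drives the round lifecycle from pre-start countdown through play to round end.
; A server-only tick, noted as once per second, counts down, asks the gamemode to start, then advances round time and reports the time limit.
; Clients get RoundStarted through the phase's RepNotify, while the gamemode's round-end event is multicast with its reason.
; The round-start binding exists but is never called.
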(event `OnRoundEnded`
  (params (Reason :type String))
  (`self.Multicast-RoundEnd` Reason)
  (set `self.RoundInProgress` "NewEnumerator2"))

(event `Multicast-RoundEnd`
  (params (Reason :type String))
  (`self.RoundEnded` Reason))

(event `OnRoundStarted`
  (set `self.RoundInProgress` "NewEnumerator0"))

(event `self.ReceiveBeginPlay`
  (`/Engine/EditorBlueprintResources/ActorMacros.Switch Has Authority`
    (:`Authority`
      (add `/Game/Blueprints/Game/BP_BaseGameMode.RoundEnded` (`/Game/Blueprints/Libs/Functions/BP_Functions_GlobalGetters.GetGamemode`) (delegate `OnRoundEnded`)))))

(event `self.ReceiveTick`
  (params (DeltaSeconds :type "Float (single-precision)"))
  (`/Engine/EditorBlueprintResources/ActorMacros.Switch Has Authority`
    (:`Authority`
      (switch `/Game/Data/Enums/E_GameState` (`self.RoundInProgress`)
        (:`NewEnumerator0`
          (bind _result (`/Engine/EditorBlueprintResources/StandardMacros.DecrementInt` (`self.RoundStartTime`))
            (:`  `
              (if (<= _result 0)
                (`/Game/Blueprints/Game/BP_BaseGameMode.StartRound` (`/Game/Blueprints/Libs/Functions/BP_Functions_GlobalGetters.GetGamemode`))
                (set `self.RoundInProgress` "NewEnumerator1")))))
        (:`NewEnumerator1`
          (`self.RoundTimeTick`))))))

(fn `OnRep_RoundInProgress`
  (switch `/Game/Data/Enums/E_GameState` (`self.RoundInProgress`)
    (:`NewEnumerator1`
      (`self.RoundStarted`))))

(fn `RoundTimeTick`
  (set `self.RoundTime` (+ (`self.RoundTime`) (`KismetMathLibrary.MakeTimespan` 0 0 0 1))) ; +1 sec to round time
  (if (and (>= (`self.RoundTime`) (`/Game/Blueprints/Game/BP_BaseGameMode.TimeLimit` (`/Game/Blueprints/Libs/Functions/BP_Functions_GlobalGetters.GetGamemode`))) (`|EnumEquality` (`self.RoundInProgress`) "NewEnumerator1"))
    (`/Game/Blueprints/Game/BP_BaseGameMode.TimeLimitReached` (`/Game/Blueprints/Libs/Functions/BP_Functions_GlobalGetters.GetGamemode`))))

(fn `UserConstructionScript`)