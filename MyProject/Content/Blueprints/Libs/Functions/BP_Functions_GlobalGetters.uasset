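; Blueprint function library of global getters that return the project's gameplay framework objects already cast to their custom classes.
; It covers the base and team game modes, the base game state, a controller's base or team player state, and a pawn's player controller.
; IsAntoterTeam builds on the team player state getter to report whether two controllers belong to different teams.
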(fn `GetCharactersController`
  (params (Pawn :type "Pawn Object Reference"))
  (returns (PlayerController :type "/Game/Blueprints/Player/BP_PlayerController Object Reference"))
  (return (cast `/Game/Blueprints/Player/BP_PlayerController` (`Pawn.GetController` Pawn) :!pure true)))

(fn `GetGamemode`
  (returns (Gamemode :type "/Game/Blueprints/Game/BP_BaseGameMode Object Reference"))
  (return (cast `/Game/Blueprints/Game/BP_BaseGameMode` (`GameplayStatics.GetGameMode` null) :!pure true)))

(fn `GetGameState`
  (returns (Out :type "/Game/Blueprints/Game/BP_BaseGameState Object Reference"))
  (return (cast `/Game/Blueprints/Game/BP_BaseGameState` (`GameplayStatics.GetGameState` null) :!pure true)))

(fn `GetPlayerStateByController`
  (params (Controller :type "Controller Object Reference"))
  (returns (`Playe State` :type "/Game/Blueprints/Player/BP_PlayerState Object Reference"))
  (return (cast `/Game/Blueprints/Player/BP_PlayerState` (`Controller.PlayerState` Controller) :!pure true)))

(fn `GetTeamGamemode`
  (returns (Gamemode :type "/Game/Blueprints/Game/BP_BaseGameMode Object Reference"))
  (return (cast `/Game/Blueprints/Game/BP_TeamGameMode` (`GameplayStatics.GetGameMode` null) :!pure true)))

(fn `GetTeamPlayerStateByController`
  (params (Controller :type "Controller Object Reference"))
  (returns (`Playe State` :type "/Game/Blueprints/Player/BP_TeamPlayerState Object Reference"))
  (return (cast `/Game/Blueprints/Player/BP_TeamPlayerState` (`Controller.PlayerState` Controller) :!pure true)))

(fn `IsAntoterTeam`
  (params (Player :type "Controller Object Reference") (OtherPlayer :type "Controller Object Reference"))
  (returns (Out :type Boolean))
  (return (`|EnumInequality` (`/Game/Blueprints/Player/BP_TeamPlayerState.Team` (`self.GetTeamPlayerStateByController` Player)) (`/Game/Blueprints/Player/BP_TeamPlayerState.Team` (`self.GetTeamPlayerStateByController` OtherPlayer)))))