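; Minimap helper actor that captures a map image of a square area and converts world positions into 2D map coordinates.
; Construction sizes the bounds box and orthographic capture width from MapSize; CaptureMapImage triggers the scene capture.
; Conversion measures from a corner of the area in the actor's rotated frame, and GetPlayerCoordinates applies it to every BP_PlayerCharacter.
; Construction also draws a debug sphere by round-tripping a hard-coded test point.
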(event `CaptureMapImage`
  (`SceneCaptureComponent2D.CaptureScene` (`self.SceneCaptureComponent2D`)))

(fn `ConvertWorldToMapLocation`
  (params (WorldLocation :type "Vector Structure"))
  (returns (Maplocation :type "Vector2D Structure"))
  (bind _returnvalue (/ (`self.MapSize`) 2.0))
  (return (`KismetMathLibrary.Conv_VectorToVector2D` (* (`KismetMathLibrary.LessLess_VectorRotator` (- (- (`self.K2_GetActorLocation`) (`KismetMathLibrary.GreaterGreater_VectorRotator` (`KismetMathLibrary.MakeVector` (* _returnvalue -1.0) _returnvalue) (`self.K2_GetActorRotation`))) WorldLocation) (`self.K2_GetActorRotation`)) (1.0 -1.0 0.0)))))

(fn `GetPlayerCoordinates`
  (returns (PlayersLocations :type "Map of /Game/Blueprints/Player/BP_PlayerCharacter Object Reference to Vector2D Structure"))
  (locals (L_PlayerCoords :type "Map of /Game/Blueprints/Player/BP_PlayerCharacter Object Reference to Vector2D Structure"))
  (bind _outactors (`GameplayStatics.GetAllActorsOfClass` "/Game/Blueprints/Player/BP_PlayerCharacter.BP_PlayerCharacter_C"))
  (for _array_element _outactors
    (`BlueprintMapLibrary.Map_Add` (`local.L_PlayerCoords`) _array_element (`self.ConvertWorldToMapLocation` (`self.K2_GetActorLocation` _array_element))))
  (return (`local.L_PlayerCoords`)))

(fn `UserConstructionScript`
  (bind _returnvalue (/ (`self.MapSize`) 2.0))
  (bind _returnvalue_2 (/ (`self.MapSize`) 2.0))
  (`BoxComponent.SetBoxExtent` (`self.Box`) (`KismetMathLibrary.MakeVector` 2.0 _returnvalue _returnvalue) true)
  (set `SceneCaptureComponent2D.OrthoWidth` (`self.MapSize`) (`self.SceneCaptureComponent2D`))
  (`KismetSystemLibrary.DrawDebugSphere` (+ (`KismetMathLibrary.GreaterGreater_VectorRotator` (* (`KismetMathLibrary.Conv_Vector2DToVector` (`self.ConvertWorldToMapLocation` (`KismetMathLibrary.MakeVector` 1685.062744 133.758698))) (-1.0 1.0 0.0)) (`self.K2_GetActorRotation`)) (- (`self.K2_GetActorLocation`) (`KismetMathLibrary.GreaterGreater_VectorRotator` (`KismetMathLibrary.MakeVector` (* _returnvalue_2 -1.0) _returnvalue_2) (`self.K2_GetActorRotation`)))) 100.0 12 (struct :`R` 1.0 :`G` 1.0 :`B` 1.0 :`A` 1.0) 0.0 20.0))