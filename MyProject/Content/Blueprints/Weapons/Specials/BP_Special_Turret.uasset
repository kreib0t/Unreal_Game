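; Deployable turret special weapon that automatically damages player characters inside its radius, skipping its instigator and, in team gamemodes, the instigator's teammates.
; The radius overlap sets a single Target and runs a looping timer that applies damage directly, without traces or projectiles, retargeting when that target leaves.
; Clients destroy the radius component, leaving detection to the authority, and only they rotate the separate yaw and pitch platforms toward the Target on Tick.
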(event `self.ReceiveTick`
  (params (DeltaSeconds :type "Float (single-precision)"))
  (`parent.ReceiveTick` DeltaSeconds)
  (`/Engine/EditorBlueprintResources/ActorMacros.Switch Has Authority`
    (:`Remote`
      (bind _target (`self.Target`)
        (:`then`
          (bind (_returnvalue_roll _returnvalue_pitch _returnvalue_yaw) (`KismetMathLibrary.BreakRotator` (`KismetMathLibrary.FindLookAtRotation` (`SceneComponent.K2_GetComponentLocation` (`self.PitchPlatform`)) (`self.K2_GetActorLocation` _target))))
          (`SceneComponent.K2_SetWorldRotation` (`self.YawPlatform`) (`KismetMathLibrary.MakeRotator` 0.0 0.0 _returnvalue_yaw) false false)
          (`SceneComponent.K2_SetRelativeRotation` (`self.PitchPlatform`) (`KismetMathLibrary.MakeRotator` 0.0 _returnvalue_pitch) false false))
        (:`else`)))))

(event `self.ReceiveBeginPlay`
  (`parent.ReceiveBeginPlay`)
  (`/Engine/EditorBlueprintResources/ActorMacros.Switch Has Authority`
    (:`Remote`
      (`ActorComponent.K2_DestroyComponent` (`self.Radius`)))))

(event `self.Radius.OnComponentBeginOverlap`
  (params (OverlappedComponent :type "PrimitiveComponent Object Reference") (OtherActor :type "Actor Object Reference") (OtherComp :type "PrimitiveComponent Object Reference") (OtherBodyIndex :type Integer) (bFromSweep :type Boolean) (SweepResult :type "HitResult Structure (by ref)"))
  (bind _asbp_player_character (cast `/Game/Blueprints/Player/BP_PlayerCharacter` OtherActor))
  (`self.Target`
    (:`then`)
    (:`else`
      (if (`self.ShouldAlarmOnCharacter` _asbp_player_character)
        (set `self.Target` _asbp_player_character)
        (`self.StartShoot`)))))

(event `self.Radius.OnComponentEndOverlap`
  (params (OverlappedComponent :type "PrimitiveComponent Object Reference") (OtherActor :type "Actor Object Reference") (OtherComp :type "PrimitiveComponent Object Reference") (OtherBodyIndex :type Integer))
  (if (== OtherActor (`self.Target`))
    (set `self.Target` null)
    (`self.StopShoot`)
    (`self.FindNewTarget`)))

(fn `FindNewTarget`
  (for _array_element (`PrimitiveComponent.GetOverlappingActors` (`self.Radius`) "/Game/Blueprints/Player/BP_PlayerCharacter.BP_PlayerCharacter_C")
    (bind _asbp_player_character (cast `/Game/Blueprints/Player/BP_PlayerCharacter` _array_element :!pure true))
    (if (`self.ShouldAlarmOnCharacter` _asbp_player_character)
      (set `self.Target` _asbp_player_character)
      (`self.StartShoot`)
      (return))))

(fn `Shoot`
  (`GameplayStatics.ApplyDamage` (`self.Target`) (`self.Damage`) (`self.GetInstigatorController`) self))

(fn `ShouldAlarmOnCharacter`
  (params (Character :type "/Game/Blueprints/Player/BP_PlayerCharacter Object Reference"))
  (returns (Out :type Boolean))
  (bind _instigator (`self.Instigator`)
    (:`then`
      (if (== _instigator Character)
        (return false)
        (else
          (`/Engine/EditorBlueprintResources/StandardMacros.IsValid` (`/Game/Blueprints/Libs/Functions/BP_Functions_GlobalGetters.GetTeamGamemode`)
            (:`Is Valid`
              (return (`/Game/Blueprints/Libs/Functions/BP_Functions_GlobalGetters.IsAntoterTeam` (`self.GetInstigatorController`) (`Pawn.GetController` Character))))
            (:`Is Not Valid`
              (return true))))))
    (:`else`
      (return true))))

(fn `StartShoot`
  (bind _returnvalue (`KismetSystemLibrary.K2_SetTimer` null "Shoot" (`self.ShootDelay`) true))
  (set `self.ShootTimer` _returnvalue))

(fn `StopShoot`
  (`KismetSystemLibrary.K2_ClearAndInvalidateTimerHandle` (`self.ShootTimer`)))

(fn `UserConstructionScript`
  (`parent.UserConstructionScript`))