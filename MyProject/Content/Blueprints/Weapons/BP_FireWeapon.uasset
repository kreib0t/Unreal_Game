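; Firearm Blueprint that extends a parent weapon with hitscan firing, ammo and timed reloading.
; When the parent use succeeds and no projectile class is set, a sphere trace from the player camera along the owner's forward vector applies point damage, with debug drawing.
; Firing on empty sets Reloading, whose RepNotify runs a server-side timer that refills ammo from the reserve; firing is blocked meanwhile.
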(event `DEBUG_DrawServerTrace`
  (params (Start :type "Vector Structure") (End :type "Vector Structure") (Hit :type "Vector Structure"))
  (`KismetSystemLibrary.DrawDebugLine` Start End (struct :`R` 0.52448 :`G` 1.0 :`A` 1.0) 5.0 2.0)
  (`KismetSystemLibrary.DrawDebugSphere` Hit 40.0 8 (struct :`R` 0.908962 :`B` 1.0 :`A` 1.0) 5.0 2.0))

(fn `AbleToReload`
  (returns (ReturnValue :type Boolean))
  (return (and (!= (defaults `/Game/Blueprints/Weapons/BP_FireWeapon` (`GameplayStatics.GetObjectClass` self)) (`self.CurrentAmmo`)) (> (`self.TotalAmmo`) 0) (not (`KismetSystemLibrary.K2_IsValidTimerHandle` (`self.ReloadTimer`))))))

(fn `AbleToUseWeapon`
  (returns (Out :type Boolean))
  (return (and (`parent.AbleToUseWeapon`) (not (`self.Reloading`)))))

(fn `GetFireTrace`
  (returns (Hit :type "HitResult Structure"))
  (bind _asbp_player_character (cast `/Game/Blueprints/Player/BP_PlayerCharacter` (`self.GetInstigator`))
    (:`then`
      (bind _returnvalue (`SceneComponent.K2_GetComponentLocation` (`/Game/Blueprints/Player/BP_PlayerCharacter.Camera` _asbp_player_character)))
      (bind _outhit (`KismetSystemLibrary.SphereTraceSingleForObjects` _returnvalue (+ _returnvalue (* (`self.GetActorForwardVector` (`self.GetOwner`)) 10000.0)) 0.0 (`|MakeArray` "ObjectTypeQuery1" "ObjectTypeQuery2" "ObjectTypeQuery3" :!type "EObjectTypeQuery Enum") false (`|MakeArray` self (`self.GetInstigator`) :!type "Actor Object Reference")))
      (bind (_bblockinghit _binitialoverlap _time _distance _location _impactpoint _normal _impactnormal _physmat _hitactor _hitcomponent _hitbonename _hititem _faceindex _tracestart _traceend) (`GameplayStatics.BreakHitResult` _outhit))
      (`self.DEBUG_DrawServerTrace` _tracestart _traceend _location)
      (return _outhit))
    (:`CastFailed`
      (return))))

(fn `OnRep_Reloading`
  (`/Engine/EditorBlueprintResources/ActorMacros.Switch Has Authority`
    (:`Authority`
      (if (`self.Reloading`)
        (if (`self.AbleToReload`)
          (`/Game/Blueprints/Libs/BP_Functions_DEbug.PrintMessage` "Reloading" (struct :`R` 0.117753 :`G` 0.383703 :`B` 0.921875 :`A` 1.0) 2.0)
          (bind _returnvalue (`KismetSystemLibrary.K2_SetTimer` null "ReloadFinished" (`self.ReloadTime`)))
          (set `self.ReloadTimer` _returnvalue)
          (set `self.AmmoToReload` (`KismetMathLibrary.Min` (- (defaults `/Game/Blueprints/Weapons/BP_FireWeapon` (`GameplayStatics.GetObjectClass` self)) (`self.CurrentAmmo`)) (`self.TotalAmmo`)))
          (else
            (set `self.Reloading` false)
            (`/Game/Blueprints/Libs/BP_Functions_DEbug.PrintMessage` "Not able to reloading" (struct :`R` 0.016927 :`G` 0.253775 :`B` 0.40625 :`A` 1.0) 2.0 true)))
        (else
          (`KismetSystemLibrary.K2_ClearAndInvalidateTimerHandle` (`self.ReloadTimer`)))))))

(fn `ReloadFinished`
  (set `self.Reloading` false)
  (set `self.CurrentAmmo` (+ (`self.AmmoToReload`) (`self.CurrentAmmo`)))
  (set `self.TotalAmmo` (- (`self.TotalAmmo`) (`self.AmmoToReload`))))

(fn `UserConstructionScript`
  (`parent.UserConstructionScript`))

(fn `UseWeapon`
  (returns (Used :type Boolean))
  (bind _used (`parent.UseWeapon`))
  (`/Game/Blueprints/Libs/BP_Functions_DEbug.PrintMessage` (`KismetStringLibrary.Concat_StrStr` (`KismetStringLibrary.Conv_IntToString` (`self.CurrentAmmo`)) "|" (`KismetStringLibrary.Conv_IntToString` (`self.TotalAmmo`))) (struct :`A` 1.0) 1.0)
  (if _used
    (if (`KismetSystemLibrary.IsValidClass` (`self.FireProjectile`))
      (return true)
      (else
        (bind _hit (`self.GetFireTrace`))
        (bind (_bblockinghit _binitialoverlap _time _distance _location _impactpoint _normal _impactnormal _physmat _hitactor _hitcomponent _hitbonename _hititem _faceindex _tracestart _traceend) (`GameplayStatics.BreakHitResult` _hit))
        (`GameplayStatics.ApplyPointDamage` _hitactor (`self.Damage`) (`KismetMathLibrary.GetDirectionUnitVector` _traceend _tracestart) _hit (`self.GetInstigatorController`) self)
        (return true)))
    (elif (and (<= (`self.CurrentAmmo`) 0) (> (`self.TotalAmmo`) 0))
      (set `self.Reloading` true)
      (return false)
      (else
        (return false)))))