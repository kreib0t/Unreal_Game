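; Special weapon that places an actor of its configured class, passing it the weapon's damage, when the parent's use check succeeds.
; While it is the current weapon, non-authority instances show a collision-free preview of that actor at a short camera trace hit, destroying it on switch.
; Placement runs its own trace from above the owner along the controller's forward vector, so it can differ from the preview.
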(event `self.ReceiveTick`
  (params (DeltaSeconds :type "Float (single-precision)"))
  (bind _camera (`/Game/Blueprints/Player/BP_PlayerCharacter.Camera` (`self.WeaponOwner`)))
  (bind _returnvalue (`SceneComponent.K2_GetComponentLocation` _camera))
  (`parent.ReceiveTick` DeltaSeconds)
  (`/Engine/EditorBlueprintResources/ActorMacros.Switch Has Authority`
    (:`Remote`
      (`self.WeaponOwner`
        (:`then`
          (if (== (`/Game/Blueprints/Components/Player/BP_WeaponManager.CurrentWeapon` (`/Game/Blueprints/Player/BP_PlayerCharacter.BP_WeaponManager` (`self.WeaponOwner`))) self)
            (`self.SpecialBeforeSet`
              (:`then`
                (bind _outhit (`KismetSystemLibrary.LineTraceSingle` _returnvalue (+ _returnvalue (* (`SceneComponent.GetForwardVector` _camera) 500.0)) "TraceTypeQuery1"))
                (`self.K2_SetActorTransform` (`self.SpecialBeforeSet`) (`KismetMathLibrary.MakeTransform` (`.Location` (`GameplayStatics.BreakHitResult` _outhit)) (`KismetMathLibrary.Conv_VectorToRotator` (`self.GetActorForwardVector` (`self.WeaponOwner`)))) false false))
              (:`else`
                (bind _returnvalue_2 (`|SpawnActorFromClass` (`self.SpecialClass`) (`KismetMathLibrary.MakeTransform` (0.0 0.0 0.0)) "AlwaysSpawn" "OverrideRootScale" null 0.0 null))
                (bind _output_get (set `self.SpecialBeforeSet` _returnvalue_2))
                (`self.SetActorEnableCollision` _output_get false)))
            (else
              (bind _specialbeforeset (`self.SpecialBeforeSet`)
                (:`then`
                  (`self.K2_DestroyActor` _specialbeforeset))
                (:`else`)))))
        (:`else`)))))

(fn `SetSpecial`
  (bind _weaponowner (`self.WeaponOwner`))
  (bind _returnvalue (+ (`self.K2_GetActorLocation` _weaponowner) (0.0 0.0 50.0)))
  (bind _outhit (`KismetSystemLibrary.LineTraceSingle` _returnvalue (+ _returnvalue (* (`self.GetActorForwardVector` (`Pawn.GetController` _weaponowner)) 500.0)) "TraceTypeQuery1"))
  (`|SpawnActorFromClass` (`self.SpecialClass`) (`KismetMathLibrary.MakeTransform` (`.Location` (`GameplayStatics.BreakHitResult` _outhit)) (`self.K2_GetActorRotation` (`self.WeaponOwner`))) "AlwaysSpawn" "OverrideRootScale" self (`self.Damage`) (`self.GetInstigator`)))

(fn `UserConstructionScript`
  (`parent.UserConstructionScript`))

(fn `UseWeapon`
  (returns (Used :type Boolean))
  (bind _used (`parent.UseWeapon`))
  (if _used
    (`self.SetSpecial`)
    (return true)
    (else
      (return false))))