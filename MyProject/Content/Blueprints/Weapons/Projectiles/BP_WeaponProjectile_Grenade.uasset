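; Grenade weapon projectile that is thrown as a physics body and explodes after a timed delay in a networked game.
; On BeginPlay the server applies a forward impulse with random spin to the box and starts the fuse timer.
; Explode deals full radial damage and destroys the actor, with remote machines spawning explosion particles on Destroyed.
; An unused team-damage trace remains; its comment defers that filtering to the health component.
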(event `self.ReceiveDestroyed`
  (`parent.ReceiveDestroyed`)
  (`/Engine/EditorBlueprintResources/ActorMacros.Switch Has Authority`
    (:`Remote`
      (`GameplayStatics.SpawnEmitterAtLocation` "/Game/Assets/StarterContent/Particles/P_Explosion.P_Explosion" (`self.K2_GetActorLocation`)))))

(event `self.ReceiveBeginPlay`
  (`/Engine/EditorBlueprintResources/ActorMacros.Switch Has Authority`
    (:`Authority`
      (`PrimitiveComponent.AddImpulse` (`self.Box`) (* (`self.GetActorForwardVector`) (`self.ThrowPower`)) "None" false)
      (`PrimitiveComponent.AddAngularImpulseInDegrees` (`self.Box`) (`KismetMathLibrary.MakeVector` (`KismetMathLibrary.RandomFloatInRange` -500.0 500.0) (`KismetMathLibrary.RandomFloatInRange` -500.0 500.0) (`KismetMathLibrary.RandomFloatInRange` -500.0 500.0)) "None" false)
      (`KismetSystemLibrary.K2_SetTimer` null "Explode" (`self.ExplotionDelay`)))))

(fn `Explode`
  (locals (L_Ignore :type "Array of Actor Object Reference"))
  (`GameplayStatics.ApplyRadialDamage` (`self.Damage`) (`self.K2_GetActorLocation`) (`self.ExplotionRadius`) null (`local.L_Ignore`) self (`self.GetInstigatorController`) true "ECC_WorldStatic")
  (`self.K2_DestroyActor`))

(fn `UserConstructionScript`
  (`parent.UserConstructionScript`))