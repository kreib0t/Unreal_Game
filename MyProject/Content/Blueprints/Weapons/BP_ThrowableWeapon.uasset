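; Throwable weapon that spawns a projectile from the player character, either immediately or after a required hold time.
; When the parent's use check passes, hold-to-throw weapons start a timer that calls ThrowGrenade.
; Stopping use before it fires cancels the throw and refunds one ammo.
; The projectile spawns ahead of the camera location along the owner's forward vector with a rotation offset, receiving the weapon's damage and instigator.
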(event `self.StopUseWeapon`
  (`parent.StopUseWeapon`)
  (if (`KismetSystemLibrary.K2_IsValidTimerHandle` (`self.ThrowGrenadeTimer`))
    (`KismetSystemLibrary.K2_ClearAndInvalidateTimerHandle` (`self.ThrowGrenadeTimer`))
    (`/Engine/EditorBlueprintResources/StandardMacros.IncrementInt` (`self.CurrentAmmo`))))

(fn `ThrowGrenade`
  (`KismetSystemLibrary.K2_ClearAndInvalidateTimerHandle` (`self.ThrowGrenadeTimer`))
  (bind _asbp_player_character (cast `/Game/Blueprints/Player/BP_PlayerCharacter` (`self.GetInstigator`)))
  (`|SpawnActorFromClass` (`self.Projectile`) (`KismetMathLibrary.MakeTransform` (+ (`SceneComponent.K2_GetComponentLocation` (`/Game/Blueprints/Player/BP_PlayerCharacter.Camera` _asbp_player_character)) (* (`self.GetActorForwardVector` (`self.GetOwner`)) 70.0)) (`KismetMathLibrary.ComposeRotators` (`KismetMathLibrary.Conv_VectorToRotator` (`self.GetActorForwardVector` (`self.GetOwner`))) (struct :`Pitch` 10.0))) "Undefined" "OverrideRootScale" self (`self.Damage`) (`self.GetInstigator`)))

(fn `UserConstructionScript`
  (`parent.UserConstructionScript`))

(fn `UseWeapon`
  (returns (Used :type Boolean))
  (bind _used (`parent.UseWeapon`))
  (if _used
    (if (`self.MustHoldToThrow`)
      (bind _returnvalue (`KismetSystemLibrary.K2_SetTimer` null "ThrowGrenade" (`self.HoldTime`)))
      (set `self.ThrowGrenadeTimer` _returnvalue)
      (return true)
      (else
        (`self.ThrowGrenade`)))
    (else
      (return false))))